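; Door actor that opens when the first-person character enters its collision box while Unlocked is set, and reverses when the character leaves.
; A timeline drives the DoorCenter component's relative location and rotation by lerping between the MarkerClose and MarkerOpen component transforms.
; The exit reversal does not check the lock.
; On BeginPlay the door also creates a HUD widget and adds it to the viewport.
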(event `self.ReceiveBeginPlay`
  (bind _returnvalue (`|CreateWidget` "/Game/Grupy/Wieczorowa/MBohatkiewicz/HUD.HUD_C"))
  (`UserWidget.AddToViewport` _returnvalue 0))

(event `self.BoxCollision.OnComponentBeginOverlap`
  (params (OverlappedComponent :type "PrimitiveComponent Object Reference") (OtherActor :type "Actor Object Reference") (OtherComp :type "PrimitiveComponent Object Reference") (OtherBodyIndex :type Integer) (bFromSweep :type Boolean) (SweepResult :type "HitResult Structure (by ref)"))
  (bind _markeropen (`self.MarkerOpen`))
  (bind _markerclose (`self.MarkerClose`))
  (bind _doorcenter (`self.DoorCenter`))
  (if (`self.Unlocked`)
    (cast `/Game/FirstPersonBP/Blueprints/FirstPersonCharacter` OtherActor)
    (bind (_direction _newtrack_0) (`Timeline|DoorOpenAnimLoc` :!label _label)
      (:`Update`
        (`SceneComponent.K2_SetRelativeLocation` _doorcenter (`KismetMathLibrary.VLerp` (`SceneComponent.RelativeLocation` _markerclose) (`SceneComponent.RelativeLocation` _markeropen) _newtrack_0) false false)
        (`SceneComponent.K2_SetRelativeRotation` _doorcenter (`KismetMathLibrary.RLerp` (`SceneComponent.RelativeRotation` _markerclose) (`SceneComponent.RelativeRotation` _markeropen) _newtrack_0) false false)))))

(event `self.BoxCollision.OnComponentEndOverlap`
  (params (OverlappedComponent :type "PrimitiveComponent Object Reference") (OtherActor :type "Actor Object Reference") (OtherComp :type "PrimitiveComponent Object Reference") (OtherBodyIndex :type Integer))
  (cast `/Game/FirstPersonBP/Blueprints/FirstPersonCharacter` OtherActor)
  (goto _label :!via `Reverse`))

(fn `UserConstructionScript`)