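; BP_TextTrigger is a trigger volume that shows on-screen text while the first-person player stands inside it.
; On BeginPlay it creates a UI_TextBox widget and fills its text block with the TextToShow variable.
; The Box overlap events add the widget to the viewport on entry, if not already shown, and remove it on exit, reacting only to FirstPersonCharacter.
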(event `self.ReceiveBeginPlay`
  (bind _returnvalue (`|CreateWidget` "/Game/FirstPersonBP/Blueprints/UI_TextBox.UI_TextBox_C"))
  (set `self.WidgetRef` _returnvalue)
  (`TextBlock.SetText` (`/Game/FirstPersonBP/Blueprints/UI_TextBox.TextBlock_107` _returnvalue) (`self.TextToShow`)))

(event `self.Box.OnComponentBeginOverlap`
  (params (OverlappedComponent :type "PrimitiveComponent Object Reference") (OtherActor :type "Actor Object Reference") (OtherComp :type "PrimitiveComponent Object Reference") (OtherBodyIndex :type Integer) (bFromSweep :type Boolean) (SweepResult :type "HitResult Structure (by ref)"))
  (cast `/Game/FirstPersonBP/Blueprints/FirstPersonCharacter` OtherActor)
  (if (not (`Widget.IsInViewport` (`self.WidgetRef`)))
    (`UserWidget.AddToViewport` (`self.WidgetRef`) 0)))

(event `self.Box.OnComponentEndOverlap`
  (params (OverlappedComponent :type "PrimitiveComponent Object Reference") (OtherActor :type "Actor Object Reference") (OtherComp :type "PrimitiveComponent Object Reference") (OtherBodyIndex :type Integer))
  (cast `/Game/FirstPersonBP/Blueprints/FirstPersonCharacter` OtherActor)
  (`Widget.RemoveFromParent` (`self.WidgetRef`)))

(fn `UserConstructionScript`)