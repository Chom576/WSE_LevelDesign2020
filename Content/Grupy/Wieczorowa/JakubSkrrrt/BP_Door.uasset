(event `self.Box.OnComponentBeginOverlap`
  (params (OverlappedComponent :type "PrimitiveComponent Object Reference") (OtherActor :type "Actor Object Reference") (OtherComp :type "PrimitiveComponent Object Reference") (OtherBodyIndex :type Integer) (bFromSweep :type Boolean) (SweepResult :type "HitResult Structure (by ref)"))
  (bind _asfirst_person_character (cast `/Game/FirstPersonBP/Blueprints/FirstPersonCharacter` OtherActor))
  (if (`self.Unlocked?`)
    (bind (_direction _newtrack_0) (`Timeline|DoorAnimation` :!label _label)
      (:`Update`
        (`SceneComponent.K2_SetRelativeLocation` (`self.Door`) (`KismetMathLibrary.VLerp` (`SceneComponent.RelativeLocation` (`self.MarkerClodesDoor`)) (`SceneComponent.RelativeLocation` (`self.MarkerOpenDoor`)) _newtrack_0) false false)))
    (elif (`/Game/FirstPersonBP/Blueprints/FirstPersonCharacter.GotKey?` _asfirst_person_character)
      (set `/Game/FirstPersonBP/Blueprints/FirstPersonCharacter.GotKey?` false _asfirst_person_character)
      (set `self.Unlocked?` true)
      (goto _label)
      (else
        (`KismetSystemLibrary.PrintString` "Nie masz klucza")))))

(event `self.Box.OnComponentEndOverlap`
  (params (OverlappedComponent :type "PrimitiveComponent Object Reference") (OtherActor :type "Actor Object Reference") (OtherComp :type "PrimitiveComponent Object Reference") (OtherBodyIndex :type Integer))
  (cast `/Game/FirstPersonBP/Blueprints/FirstPersonCharacter` OtherActor)
  (goto _label :!via `Reverse`))

(fn `UserConstructionScript`)